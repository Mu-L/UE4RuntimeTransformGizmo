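; BP_CameraTarget_Test is a test orbit camera target that sends the shared camera pawn into a transition to its location and orbit settings.
; On enter, it passes rotation, zoom and focal length to StartCameraTransition, using either saved values or its defaults depending on ShouldSaveTransform.
; On exit, it caches those three values from the pawn only if the pawn is in the Orbiting state.
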(event `/Game/Mytaverse/OrbitCamera/BPI_CameraTarget.InitCamera`
  (params (Manager :type "/Game/Mytaverse/OrbitCamera/BP_CameraTransitionManager Object Reference"))
  (bind ((`OrbitLocation_48_BF1412AF49F7725AD2EEBBBF5DC15FD3` _orbitlocation) (`ZoomDistance_7_4B8FF0D84D06DB56580A7CADC89D6A89` _zoomdistance) (`FocalLength_27_A06297E0472BF47126912399589F048A` _focallength)) (break `/Game/Mytaverse/OrbitCamera/FOrbitCameraSettings` (`self.OrbitCameraSettings`)))
  (`parent.InitCamera` Manager)
  (set `self.SavedOrbitRotation` (`self.K2_GetActorRotation`))
  (set `self.SavedZoomDistance` _zoomdistance)
  (set `self.SavedFocalLength` _focallength))

(event `/Game/Mytaverse/OrbitCamera/BPI_CameraTarget.EnterCamera`
  (bind _orbitcamerasettings (`self.OrbitCameraSettings`))
  (bind _bshouldsavetransform (`self.bShouldSaveTransform`))
  (bind ((`ZoomDistance_7_4B8FF0D84D06DB56580A7CADC89D6A89` _zoomdistance) (`FocalLength_27_A06297E0472BF47126912399589F048A` _focallength)) (break `/Game/Mytaverse/OrbitCamera/FOrbitCameraSettings` _orbitcamerasettings))
  (`parent.EnterCamera`)
  (bind _structout (setmembers `/Game/Mytaverse/OrbitCamera/FOrbitCameraSettings` :`StructRef` _orbitcamerasettings :`OrbitLocation` (`self.K2_GetActorLocation`) :`OrbitRotation` (`KismetMathLibrary.SelectRotator` (`self.SavedOrbitRotation`) (`self.K2_GetActorRotation`) _bshouldsavetransform) :`ZoomDistance` (`KismetMathLibrary.SelectFloat` (`self.SavedZoomDistance`) _zoomdistance _bshouldsavetransform) :`FocalLength` (`KismetMathLibrary.SelectFloat` (`self.SavedFocalLength`) _focallength _bshouldsavetransform)))
  (`/Game/Mytaverse/OrbitCamera/BP_OrbitCameraPawn.StartCameraTransition` (`/Game/Mytaverse/OrbitCamera/BP_CameraTransitionManager.CameraPawn` (`self.GetTransitionManager`)) _structout))

(event `/Game/Mytaverse/OrbitCamera/BPI_CameraTarget.ExitCamera`
  (bind _camerapawn (`/Game/Mytaverse/OrbitCamera/BP_CameraTransitionManager.CameraPawn` (`self.GetTransitionManager`)))
  (`parent.ExitCamera`)
  (switch `/Game/Mytaverse/OrbitCamera/EOrbitCameraState` (`/Game/Mytaverse/OrbitCamera/BP_OrbitCameraPawn.GetCameraState` _camerapawn)
    (:`NewEnumerator0`
      (set `self.SavedOrbitRotation` (`self.K2_GetActorRotation` _camerapawn))
      (set `self.SavedZoomDistance` (`/Game/Mytaverse/OrbitCamera/BP_OrbitCameraPawn.GetZoomDistance` _camerapawn))
      (set `self.SavedFocalLength` (`/Game/Mytaverse/OrbitCamera/BP_OrbitCameraPawn.GetFocalLength` _camerapawn)))))

(event `/Game/Mytaverse/OrbitCamera/BPI_CameraTarget.TickCamera`
  (params (DeltaTime :type "Float (double-precision)"))
  (`parent.TickCamera` DeltaTime))

(fn `CanEnterFromSelf`
  (returns (ReturnValue :type Boolean))
  (return (`self.bCanEnterFromSelf`)))

(fn `UserConstructionScript`
  (`parent.UserConstructionScript`))