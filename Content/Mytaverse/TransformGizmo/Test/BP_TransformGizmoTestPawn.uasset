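; Test pawn for BP_TransformGizmo that lets a user orbit, pan and zoom the view, select actors and transform them with the gizmo.
; Mouse and touch gestures drive the camera and PointerInteraction, with orbit and mouse panning suppressed during gizmo drags.
; Releasing over no hovered object line-traces for an actor, then activates the gizmo, whose TransformEvent callback moves it.
; Hotkeys switch gizmo mode, align space and snapping; BeginPlay adds a test widget and adjusts rendering cvars.
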(event `self.ReceiveBeginPlay`
  (`parent.ReceiveBeginPlay`)
  (`KismetSystemLibrary.ExecuteConsoleCommand` "r.AntiAliasingMethod 1" null)
  (`KismetSystemLibrary.ExecuteConsoleCommand` "r.DefaultFeature.AutoExposure 0" null)
  (`KismetSystemLibrary.ExecuteConsoleCommand` "r.MotionBlur.Amount 0" null)
  (`/Game/Mytaverse/PointerInteraction/BP_PointerInteractionComponent.SetupInteraction` (`self.PointerInteraction`) (make `/Game/Mytaverse/PointerInteraction/FPointerInteractionSettings` "NewEnumerator9" 100000.0 true (`|MakeArray` "ObjectTypeQuery2" :!type "EObjectTypeQuery Enum") null) true)
  (bind _returnvalue (`|CreateWidget` "/Game/Mytaverse/TransformGizmo/Test/WBP_TransformGizmoTest.WBP_TransformGizmoTest_C"))
  (`UserWidget.AddToViewport` _returnvalue 0))

(event `self.ReceiveTick`
  (params (DeltaSeconds :type "Float (single-precision)"))
  (`parent.ReceiveTick` DeltaSeconds)
  (if (not (`/Game/Mytaverse/PointerInteraction/BP_PointerInteractionComponent.bIsDragging` (`self.PointerInteraction`)))
    (`|ExecutionSequence`
      (:`then_0`
        (if (`self.bRightMosuePressed`)
          (`self.AddOrbitInput` (`KismetMathLibrary.MakeVector2D` (`self.GetInputAxisKeyValue`) (`self.GetInputAxisKeyValue`)))
          (elif (`self.bMiddleMousePressed`)
            (`self.AddPanInput` (`KismetMathLibrary.MakeVector2D` (`self.GetInputAxisKeyValue`) (`self.GetInputAxisKeyValue`))))))
      (:`then_1`
        (`self.AddZoomInput` (`self.GetInputAxisKeyValue`))))))

(event `Key|RightMouseButton`
  (params (Key :type "Key Structure"))
  (:`Pressed`
    (set `self.bRightMosuePressed` true))
  (:`Released`
    (set `self.bRightMosuePressed` false)))

(event `Key|MiddleMouseButton`
  (params (Key :type "Key Structure"))
  (:`Pressed`
    (set `self.bMiddleMousePressed` true))
  (:`Released`
    (set `self.bMiddleMousePressed` false)))

(event `SelectActor`
  (params (RayStart :type "Vector Structure") (RayEnd :type "Vector Structure"))
  (`/Engine/EditorBlueprintResources/StandardMacros.IsValid` (`/Game/Mytaverse/PointerInteraction/BP_PointerInteractionComponent.GetHoveredObject` (`self.PointerInteraction`))
    (:`Is Not Valid`
      (bind (_outhit _returnvalue) (`KismetSystemLibrary.LineTraceSingle` RayStart RayEnd "TraceTypeQuery1"))
      (if _returnvalue
        (set `self.SelectedActor` (`.HitActor` (`GameplayStatics.BreakHitResult` _outhit)))
        (bind _returnvalue_2 (`GameplayStatics.GetActorOfClass` "/Game/Mytaverse/TransformGizmo/BP_TransformGizmo.BP_TransformGizmo_C"))
        (`/Game/Mytaverse/TransformGizmo/BP_TransformGizmo.ActivateGizmo` _returnvalue_2 (`self.GetTransform` (`self.SelectedActor`)) (delegate `TransformEvent`))))))

(event `Key|LeftMouseButton`
  (params (Key :type "Key Structure"))
  (bind (_raystart _rayend) (`/Game/Mytaverse/PointerInteraction/BP_PointerInteractionComponent.GetPointerRay` (`self.PointerInteraction`)))
  (:`Pressed`
    (`/Game/Mytaverse/PointerInteraction/BP_PointerInteractionComponent.PressPointer` (`self.PointerInteraction`)))
  (:`Released`
    (`/Game/Mytaverse/PointerInteraction/BP_PointerInteractionComponent.ReleasePointer` (`self.PointerInteraction`))
    (`self.SelectActor` _raystart _rayend)))

(event `TransformEvent`
  (params (Transform :type "Transform Structure"))
  (`self.K2_SetActorTransform` (`self.SelectedActor`) Transform false false))

(event `Key|W`
  (params (Key :type "Key Structure"))
  (:`Pressed`
    (bind _returnvalue (`GameplayStatics.GetActorOfClass` "/Game/Mytaverse/TransformGizmo/BP_TransformGizmo.BP_TransformGizmo_C"))
    (`/Game/Mytaverse/TransformGizmo/BP_TransformGizmo.SetTransformMode` _returnvalue "NewEnumerator0" false)))

(event `Key|E`
  (params (Key :type "Key Structure"))
  (:`Pressed`
    (bind _returnvalue (`GameplayStatics.GetActorOfClass` "/Game/Mytaverse/TransformGizmo/BP_TransformGizmo.BP_TransformGizmo_C"))
    (`/Game/Mytaverse/TransformGizmo/BP_TransformGizmo.SetTransformMode` _returnvalue "NewEnumerator1" false)))

(event `Key|R`
  (params (Key :type "Key Structure"))
  (:`Pressed`
    (bind _returnvalue (`GameplayStatics.GetActorOfClass` "/Game/Mytaverse/TransformGizmo/BP_TransformGizmo.BP_TransformGizmo_C"))
    (`/Game/Mytaverse/TransformGizmo/BP_TransformGizmo.SetTransformMode` _returnvalue "NewEnumerator2" false)))

(event `Key|T`
  (params (Key :type "Key Structure"))
  (:`Pressed`
    (bind _returnvalue (`GameplayStatics.GetActorOfClass` "/Game/Mytaverse/TransformGizmo/BP_TransformGizmo.BP_TransformGizmo_C"))
    (`/Game/Mytaverse/TransformGizmo/BP_TransformGizmo.SetTransformMode` _returnvalue "NewEnumerator0" true)))

(event `Key|Q`
  (params (Key :type "Key Structure"))
  (:`Pressed`
    (bind _returnvalue (`GameplayStatics.GetActorOfClass` "/Game/Mytaverse/TransformGizmo/BP_TransformGizmo.BP_TransformGizmo_C"))
    (`/Engine/EditorBlueprintResources/StandardMacros.FlipFlop`
      (:`A`
        (`/Game/Mytaverse/TransformGizmo/BP_TransformGizmo.SetAlignSpace` _returnvalue "NewEnumerator1"))
      (:`B`
        (`/Game/Mytaverse/TransformGizmo/BP_TransformGizmo.SetAlignSpace` _returnvalue "NewEnumerator0")))))

(event `Key|S`
  (params (Key :type "Key Structure"))
  (:`Pressed`
    (bind _returnvalue (`GameplayStatics.GetActorOfClass` "/Game/Mytaverse/TransformGizmo/BP_TransformGizmo.BP_TransformGizmo_C"))
    (`/Engine/EditorBlueprintResources/StandardMacros.FlipFlop`
      (:`A`
        (set `/Game/Mytaverse/TransformGizmo/BP_TransformGizmo.bEnableLocationSnap` true _returnvalue)
        (set `/Game/Mytaverse/TransformGizmo/BP_TransformGizmo.bEnableRotationSnap` true _returnvalue)
        (set `/Game/Mytaverse/TransformGizmo/BP_TransformGizmo.bEnableScaleSnap` true _returnvalue))
      (:`B`
        (set `/Game/Mytaverse/TransformGizmo/BP_TransformGizmo.bEnableLocationSnap` false _returnvalue)
        (set `/Game/Mytaverse/TransformGizmo/BP_TransformGizmo.bEnableRotationSnap` false _returnvalue)
        (set `/Game/Mytaverse/TransformGizmo/BP_TransformGizmo.bEnableScaleSnap` false _returnvalue)))))

(event `self.ReceiveEndPlay`
  (params (EndPlayReason :type "EEndPlayReason Enum" :default "Destroyed"))
  (`KismetSystemLibrary.ExecuteConsoleCommand` "r.AntiAliasingMethod 4" null)
  (`KismetSystemLibrary.ExecuteConsoleCommand` "r.DefaultFeature.AutoExposure 0" null)
  (`KismetSystemLibrary.ExecuteConsoleCommand` "r.MotionBlur.Amount 0" null))

(event `InputTouch`
  (params (Location :type "Vector Structure") (FingerIndex :type "ETouchIndex Enum"))
  ;[1 1 1] 触控分发
  (:`Pressed`
    (`/Game/Mytaverse/Blueprints/PointerTouch/BPML_PointerTouchMacros.HandleTouchInput` (`KismetMathLibrary.Conv_VectorToVector2D` Location) FingerIndex :!label _label))
  (:`Released`
    (goto _label :!via `Released`))
  (:`Moved`
    (goto _label :!via `Moved`)))

(event `self.PointerTouch.OnTapDown`
  (params (Position :type "Vector2D Structure"))
  (bind _pointerinteraction (`self.PointerInteraction`))
  ;[1 1 1] Tap
  (`/Game/Mytaverse/PointerInteraction/BP_PointerInteractionComponent.UpdateHover` _pointerinteraction)
  (`/Engine/EditorBlueprintResources/StandardMacros.IsValid` (`/Game/Mytaverse/PointerInteraction/BP_PointerInteractionComponent.GetHoveredObject` _pointerinteraction)
    (:`Is Valid`
      (`/Game/Mytaverse/PointerInteraction/BP_PointerInteractionComponent.PressPointer` (`self.PointerInteraction`)))))

(event `self.PointerTouch.OnTapUp`
  (params (Position :type "Vector2D Structure"))
  (bind (_worldposition _worlddirection) (`GameplayStatics.DeprojectScreenToWorld` (`GameplayStatics.GetPlayerController` 0) Position))
  ;[1 1 1] Tap
  (`/Game/Mytaverse/PointerInteraction/BP_PointerInteractionComponent.ReleasePointer` (`self.PointerInteraction`))
  (`self.SelectActor` _worldposition (+ _worldposition (* _worlddirection (`.InteractionDistance_5_0B771AF24CDCD6EDB7CAF593A88C4182` (break `/Game/Mytaverse/PointerInteraction/FPointerInteractionSettings` (`/Game/Mytaverse/PointerInteraction/BP_PointerInteractionComponent.InteractionSettings` (`self.PointerInteraction`))))))))

(event `self.PointerTouch.OnDragStart`
  (params (Position :type "Vector2D Structure"))
  ;[1 1 1] Drag
)

(event `self.PointerTouch.OnDragMove`
  (params (DeltaDrag :type "Vector2D Structure"))
  ;[1 1 1] Drag
  (if (not (`/Game/Mytaverse/PointerInteraction/BP_PointerInteractionComponent.bIsDragging` (`self.PointerInteraction`)))
    (`self.AddOrbitInput` (* DeltaDrag (0.1 -0.1)))))

(event `self.PointerTouch.OnDragEnd`
  (params (Position :type "Vector2D Structure"))
  ;[1 1 1] Drag
  (`/Game/Mytaverse/PointerInteraction/BP_PointerInteractionComponent.ReleasePointer` (`self.PointerInteraction`)))

(event `self.PointerTouch.OnPinchStart`
  (params (PinchCenter :type "Vector2D Structure"))
  ;[1 1 1] Pinch
)

(event `self.PointerTouch.OnPinchMove`
  (params (DeltaPan :type "Vector2D Structure") (DeltaZoom :type "Float (double-precision)"))
  ;[1 1 1] Pinch
  (`self.AddZoomInput` (* DeltaZoom 0.05))
  (`self.AddPanInput` (* DeltaPan (0.05 -0.05))))

(event `self.PointerTouch.OnPinchEnd`
  (params (PinchCenter :type "Vector2D Structure"))
  ;[1 1 1] Pinch
)

(fn `UserConstructionScript`
  (`parent.UserConstructionScript`))