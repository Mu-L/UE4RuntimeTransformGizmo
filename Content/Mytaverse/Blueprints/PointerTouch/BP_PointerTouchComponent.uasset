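; Pointer touch component that turns raw touch input into tap, drag and two-finger pinch gesture events.
; Touch press, move and release update a pointer-position map, driving a None/Press/Drag/Pinch state machine by pointer count.
; Tick compares positions with the previous frame's snapshot, starting a drag when per-frame movement exceeds DragThreshold and emitting drag deltas or pinch pan and zoom deltas.
; Gestures read only pointer indices 0 and 1.
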(event `OnTouchPress`
  (params (PointerIndex :type "Byte (by ref)") (Position :type "Vector2D Structure"))
  (bind _pointerpositions (`self.PointerPositions`))
  (bind (_value _returnvalue) (`BlueprintMapLibrary.Map_Find` (`self.PointerPositions`)))
  (bind (_value_2 _returnvalue_2) (`BlueprintMapLibrary.Map_Find` _pointerpositions))
  (bind (_value_3 _returnvalue_3) (`BlueprintMapLibrary.Map_Find` _pointerpositions 1))
  (`BlueprintMapLibrary.Map_Add` (`self.PointerPositions`) PointerIndex Position)
  (set `self.LastPointerPositions` (`self.PointerPositions`))
  (switch `int` (`self.GetPointersNum`)
    (:`1`
      (switch `/Game/Mytaverse/Blueprints/PointerTouch/EPointerTouchState` (`self.TouchState`)
        (:`NewEnumerator7`
          ;[1 1 1] 如果只有有一个触控点，且触控状态为None时，本次触控判定为进入Press状态
          (if _returnvalue
            (set `self.TouchState` "NewEnumerator12")
            (`self.OnTapDown` _value)))))
    (:`2`
      (switch `/Game/Mytaverse/Blueprints/PointerTouch/EPointerTouchState` (`self.TouchState`)
        (:`NewEnumerator7`
          _)
        (:`NewEnumerator12`
          _)
        (:`NewEnumerator4`
          (`self.OnDragEnd` (`BlueprintMapLibrary.Map_Find` (`self.PointerPositions`))) ; 如果当前触控状态为Drag，则退出Drag状态
        ))
      ;[1 1 1] 当只有有两个触控点时，则进入Pinch状态
      (if (and _returnvalue_2 _returnvalue_3)
        (set `self.TouchState` "NewEnumerator10")
        (`self.OnPinchStart` (`/Game/Mytaverse/Blueprints/CoreHelperFunctions.Vector2dMultiplyByFloat` (+ _value_2 _value_3) 0.5))))))

(event `OnTouchMove`
  (params (PointerIndex :type Byte) (Position :type "Vector2D Structure"))
  (`BlueprintMapLibrary.Map_Add` (`self.PointerPositions`) PointerIndex Position))

(event `self.ReceiveTick`
  (params (DeltaSeconds :type "Float (single-precision)"))
  (bind _lastpointerpositions (`self.LastPointerPositions`))
  (bind _pointerpositions (`self.PointerPositions`))
  (bind _pointerpositions_2 (`self.PointerPositions`))
  (bind _lastpointerpositions_2 (`self.LastPointerPositions`))
  (bind (_value _returnvalue) (`BlueprintMapLibrary.Map_Find` (`self.PointerPositions`)))
  (bind (_value_2 _returnvalue_2) (`BlueprintMapLibrary.Map_Find` (`self.LastPointerPositions`)))
  (bind (_value_3 _returnvalue_3) (`BlueprintMapLibrary.Map_Find` (`self.PointerPositions`)))
  (bind _value_4 (`BlueprintMapLibrary.Map_Find` _pointerpositions_2))
  (bind _value_5 (`BlueprintMapLibrary.Map_Find` _pointerpositions_2 1))
  (bind _value_6 (`BlueprintMapLibrary.Map_Find` _lastpointerpositions_2))
  (bind _value_7 (`BlueprintMapLibrary.Map_Find` _lastpointerpositions_2 1))
  (bind (_value_8 _returnvalue_4) (`BlueprintMapLibrary.Map_Find` (`self.LastPointerPositions`)))
  (`|ExecutionSequence`
    (:`then_0`
      (switch `int` (`self.GetPointersNum`)
        (:`1`
          (switch `/Game/Mytaverse/Blueprints/PointerTouch/EPointerTouchState` (`self.TouchState`)
            (:`NewEnumerator12`
              ;[1 1 1] 当只有一个触控点，且触控状态为Press时，如果移动超过一定范围，则进入Drag状态
              (if (and _returnvalue _returnvalue_2)
                (if (> (`KismetMathLibrary.VSize2D` (- _value _value_2)) (`self.DragThreshold`))
                  (set `self.TouchState` "NewEnumerator4")
                  (`self.OnDragStart` (`BlueprintMapLibrary.Map_Find` (`self.PointerPositions`))))))
            (:`NewEnumerator4`
              ;[1 1 1] Drag状态更新
              (if (and _returnvalue_3 _returnvalue_4)
                (`self.OnDragMove` (- _value_3 _value_8))))))
        (:`2`
          (switch `/Game/Mytaverse/Blueprints/PointerTouch/EPointerTouchState` (`self.TouchState`)
            (:`NewEnumerator10`
              ;[1 1 1] 更新Pinch状态
              (if (and (`.ReturnValue` (`BlueprintMapLibrary.Map_Find` _pointerpositions)) (`.ReturnValue` (`BlueprintMapLibrary.Map_Find` _pointerpositions 1)) (`.ReturnValue` (`BlueprintMapLibrary.Map_Find` _lastpointerpositions)) (`.ReturnValue` (`BlueprintMapLibrary.Map_Find` _lastpointerpositions 1)))
                (`self.OnPinchMove` (- (`/Game/Mytaverse/Blueprints/CoreHelperFunctions.Vector2dMultiplyByFloat` (+ _value_4 _value_5) 0.5) (`/Game/Mytaverse/Blueprints/CoreHelperFunctions.Vector2dMultiplyByFloat` (+ _value_6 _value_7) 0.5)) (- (`KismetMathLibrary.Distance2D` _value_4 _value_5) (`KismetMathLibrary.Distance2D` _value_6 _value_7)))))))))
    (:`then_1`
      (set `self.LastPointerPositions` (`self.PointerPositions`)))))

(event `OnTouchRelease`
  (params (PointerIndex :type Byte) (Position :type "Vector2D Structure"))
  (bind _pointerpositions (`self.PointerPositions`))
  (bind (_value _returnvalue) (`BlueprintMapLibrary.Map_Find` _pointerpositions))
  (bind (_value_2 _returnvalue_2) (`BlueprintMapLibrary.Map_Find` _pointerpositions 1))
  (`|ExecutionSequence`
    (:`then_0`
      (switch `int` (`self.GetPointersNum`)
        (:`1`
          (switch `/Game/Mytaverse/Blueprints/PointerTouch/EPointerTouchState` (`self.TouchState`)
            (:`NewEnumerator12`
              (if (`.ReturnValue` (`BlueprintMapLibrary.Map_Find` (`self.PointerPositions`)))
                (set `self.TouchState` "NewEnumerator7")
                (`self.OnTapUp` (`BlueprintMapLibrary.Map_Find` (`self.PointerPositions`)))))
            (:`NewEnumerator4`
              (if (`.ReturnValue` (`BlueprintMapLibrary.Map_Find` (`self.PointerPositions`)))
                (set `self.TouchState` "NewEnumerator7")
                (`self.OnDragEnd` (`BlueprintMapLibrary.Map_Find` (`self.PointerPositions`)))))))
        (:`2`
          (switch `/Game/Mytaverse/Blueprints/PointerTouch/EPointerTouchState` (`self.TouchState`)
            (:`NewEnumerator10`
              (if (and _returnvalue _returnvalue_2)
                (set `self.TouchState` "NewEnumerator7")
                (`self.OnPinchEnd` (`/Game/Mytaverse/Blueprints/CoreHelperFunctions.Vector2dMultiplyByFloat` (+ _value _value_2) 0.5))))))))
    (:`then_1`
      (`BlueprintMapLibrary.Map_Remove` (`self.PointerPositions`) PointerIndex)
      (set `self.LastPointerPositions` (`self.PointerPositions`)))))

(fn `GetPointersNum`
  (returns (ReturnValue :type Integer))
  (bind _keys (`BlueprintMapLibrary.Map_Keys` (`self.PointerPositions`)))
  (return (`KismetArrayLibrary.Array_Length` _keys)))