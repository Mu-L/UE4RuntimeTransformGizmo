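; CoreHelperFunctions is a collection of small, general-purpose helper functions for geometry, spline and string work.
; Array helpers offset 2D points, convert between 2D and 3D vectors, transform locations and gather every spline point's location in a chosen coordinate space.
; Smaller utilities supply an identity transform, scale a 2D vector by a float, provide an end-line string and zero-pad integers through text formatting.
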(fn `DefaultTransform`
  (returns (ReturnValue :type "Transform Structure"))
  (return (`KismetMathLibrary.MakeTransform` (0.0 0.0 0.0))))

(fn `EndLine`
  (returns (ReturnValue :type String))
  (return " \n"))

(fn `GetSplinePointsLocations`
  (params (Spline :type "SplineComponent Object Reference") (Coordinate :type "ESplineCoordinateSpace Enum" :default "Local"))
  (returns (ReturnValue :type "Array of Vector Structure"))
  (locals (Locations :type "Array of Vector Structure"))
  (for _index (range (`SplineComponent.GetNumberOfSplinePoints` Spline))
    (`KismetArrayLibrary.Array_Add` (`local.Locations`) (`SplineComponent.GetLocationAtSplinePoint` Spline _index Coordinate)))
  (return (`local.Locations`)))

(fn `OffsetVector2Ds`
  (params (InVector2Ds :type "Array of Vector2D Structure") (Offset :type "Vector2D Structure"))
  (returns (ReturnValue :type "Array of Vector2D Structure"))
  (locals (OutVector2Ds :type "Array of Vector2D Structure"))
  (for _array_element InVector2Ds
    (`KismetArrayLibrary.Array_Add` (`local.OutVector2Ds`) (+ _array_element Offset)))
  (return (`local.OutVector2Ds`)))

(fn `TransformLocations`
  (params (T :type "Transform Structure") (Locations :type "Array of Vector Structure"))
  (returns (ReturnValue :type "Array of Vector Structure"))
  (locals (OutLocations :type "Array of Vector Structure"))
  (for _array_element Locations
    (`KismetArrayLibrary.Array_Add` (`local.OutLocations`) (`KismetMathLibrary.TransformLocation` T _array_element)))
  (return (`local.OutLocations`)))

(fn `Vector2dMultiplyByFloat`
  (params (A :type "Vector2D Structure") (B :type "Float (double-precision)"))
  (returns (ReturnValue :type "Vector2D Structure"))
  (return (* A (`KismetMathLibrary.MakeVector2D` B B))))

(fn `Vector2DsToVectors`
  (params (InVector2Ds :type "Array of Vector2D Structure") (Z :type "Float (single-precision)"))
  (returns (ReturnValue :type "Array of Vector Structure"))
  (locals (Vectors :type "Array of Vector Structure"))
  (bind _vectors (`local.Vectors`))
  (for _array_element InVector2Ds
    (`KismetArrayLibrary.Array_Add` _vectors (`KismetMathLibrary.Conv_Vector2DToVector` _array_element Z)))
  (return _vectors))

(fn `VectorsToVector2Ds`
  (params (InVectors :type "Array of Vector Structure"))
  (returns (ReturnValue :type "Array of Vector2D Structure"))
  (locals (Vector2Ds :type "Array of Vector2D Structure"))
  (for _array_element InVectors
    (`KismetArrayLibrary.Array_Add` (`local.Vector2Ds`) (`KismetMathLibrary.Conv_VectorToVector2D` _array_element)))
  (return (`local.Vector2Ds`)))

(fn `ZeroFill`
  (params (Value :type Integer) (Count :type Integer :default 3))
  (returns (ReturnValue :type String))
  (return (`KismetTextLibrary.Conv_TextToString` (`KismetTextLibrary.Conv_IntToText` Value false false Count))))