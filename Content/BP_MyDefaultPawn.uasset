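; Test pawn that lets the player pick actors with the mouse and edit them with BP_TransformGizmo.
; Left click presses the hovered pointer target or line-traces to select an actor, activating the gizmo, whose transform event moves it.
; Keys switch transform mode and toggle align space and snapping.
; BeginPlay sets up the pointer component, cursor and test widget, and adjusts rendering console variables; EndPlay resets anti-aliasing.
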(event `self.ReceiveBeginPlay`
  (`parent.ReceiveBeginPlay`)
  (`/Game/Mytaverse/PointerInteraction/BP_PointerInteractionComponent.SetupInteraction` (`self.BP_PointerInteractionComponent`) (make `/Game/Mytaverse/PointerInteraction/FPointerInteractionSettings` "NewEnumerator9" 400000.0 true (`|MakeArray` "ObjectTypeQuery2" :!type "EObjectTypeQuery Enum") null) true)
  (set `PlayerController.bShowMouseCursor` true (`GameplayStatics.GetPlayerController` 0))
  (bind _returnvalue (`|CreateWidget` "/Game/Mytaverse/TransformGizmo/Test/WBP_TransformGizmoTest.WBP_TransformGizmoTest_C"))
  (`UserWidget.AddToViewport` _returnvalue 0)
  (`KismetSystemLibrary.ExecuteConsoleCommand` "r.AntiAliasingMethod 0" null)
  (`KismetSystemLibrary.ExecuteConsoleCommand` "r.DefaultFeature.AutoExposure 0" null)
  (`KismetSystemLibrary.ExecuteConsoleCommand` "r.MotionBlur.Amount 0" null))

(event `Key|LeftMouseButton`
  (params (Key :type "Key Structure"))
  (bind (_raystart _rayend) (`/Game/Mytaverse/PointerInteraction/BP_PointerInteractionComponent.GetPointerRay` (`self.BP_PointerInteractionComponent`)))
  (:`Pressed`
    (`/Engine/EditorBlueprintResources/StandardMacros.IsValid` (`/Game/Mytaverse/PointerInteraction/BP_PointerInteractionComponent.GetHoveredObject` (`self.BP_PointerInteractionComponent`))
      (:`Is Valid`
        (`/Game/Mytaverse/PointerInteraction/BP_PointerInteractionComponent.PressPointer` (`self.BP_PointerInteractionComponent`))
        (if (`/Game/Mytaverse/PointerInteraction/BP_PointerInteractionComponent.bIsDragging` (`self.BP_PointerInteractionComponent`))
          (`Controller.SetIgnoreLookInput` (`GameplayStatics.GetPlayerController` 0) true)))
      (:`Is Not Valid`
        (bind (_outhit _returnvalue) (`KismetSystemLibrary.LineTraceSingle` _raystart _rayend "TraceTypeQuery1"))
        (if _returnvalue
          (set `self.SelectedActor` (`.HitActor` (`GameplayStatics.BreakHitResult` _outhit)))
          (bind _returnvalue_2 (`GameplayStatics.GetActorOfClass` "/Game/Mytaverse/TransformGizmo/BP_TransformGizmo.BP_TransformGizmo_C"))
          (`/Game/Mytaverse/TransformGizmo/BP_TransformGizmo.ActivateGizmo` _returnvalue_2 (`self.GetTransform` (`self.SelectedActor`)) (delegate `TransformEvent`))))))
  (:`Released`
    (`/Game/Mytaverse/PointerInteraction/BP_PointerInteractionComponent.ReleasePointer` (`self.BP_PointerInteractionComponent`))
    (`Controller.SetIgnoreLookInput` (`GameplayStatics.GetPlayerController` 0) false)))

(event `TransformEvent`
  (params (Transform :type "Transform Structure"))
  (`self.K2_SetActorTransform` (`self.SelectedActor`) Transform false false))

(event `Key|W`
  (params (Key :type "Key Structure"))
  (:`Pressed`
    (bind _returnvalue (`GameplayStatics.GetActorOfClass` "/Game/Mytaverse/TransformGizmo/BP_TransformGizmo.BP_TransformGizmo_C"))
    (`/Game/Mytaverse/TransformGizmo/BP_TransformGizmo.SetTransformMode` _returnvalue "NewEnumerator0" false)))

(event `Key|E`
  (params (Key :type "Key Structure"))
  (:`Pressed`
    (bind _returnvalue (`GameplayStatics.GetActorOfClass` "/Game/Mytaverse/TransformGizmo/BP_TransformGizmo.BP_TransformGizmo_C"))
    (`/Game/Mytaverse/TransformGizmo/BP_TransformGizmo.SetTransformMode` _returnvalue "NewEnumerator1" false)))

(event `Key|R`
  (params (Key :type "Key Structure"))
  (:`Pressed`
    (bind _returnvalue (`GameplayStatics.GetActorOfClass` "/Game/Mytaverse/TransformGizmo/BP_TransformGizmo.BP_TransformGizmo_C"))
    (`/Game/Mytaverse/TransformGizmo/BP_TransformGizmo.SetTransformMode` _returnvalue "NewEnumerator2" false)))

(event `Key|T`
  (params (Key :type "Key Structure"))
  (:`Pressed`
    (bind _returnvalue (`GameplayStatics.GetActorOfClass` "/Game/Mytaverse/TransformGizmo/BP_TransformGizmo.BP_TransformGizmo_C"))
    (`/Game/Mytaverse/TransformGizmo/BP_TransformGizmo.SetTransformMode` _returnvalue "NewEnumerator0" true)))

(event `Key|Q`
  (params (Key :type "Key Structure"))
  (:`Pressed`
    (bind _returnvalue (`GameplayStatics.GetActorOfClass` "/Game/Mytaverse/TransformGizmo/BP_TransformGizmo.BP_TransformGizmo_C"))
    (`/Engine/EditorBlueprintResources/StandardMacros.FlipFlop`
      (:`A`
        (`/Game/Mytaverse/TransformGizmo/BP_TransformGizmo.SetAlignSpace` _returnvalue "NewEnumerator1"))
      (:`B`
        (`/Game/Mytaverse/TransformGizmo/BP_TransformGizmo.SetAlignSpace` _returnvalue "NewEnumerator0")))))

(event `Key|S`
  (params (Key :type "Key Structure"))
  (:`Pressed`
    (bind _returnvalue (`GameplayStatics.GetActorOfClass` "/Game/Mytaverse/TransformGizmo/BP_TransformGizmo.BP_TransformGizmo_C"))
    (`/Engine/EditorBlueprintResources/StandardMacros.FlipFlop`
      (:`A`
        (set `/Game/Mytaverse/TransformGizmo/BP_TransformGizmo.bEnableLocationSnap` true _returnvalue)
        (set `/Game/Mytaverse/TransformGizmo/BP_TransformGizmo.bEnableRotationSnap` true _returnvalue)
        (set `/Game/Mytaverse/TransformGizmo/BP_TransformGizmo.bEnableScaleSnap` true _returnvalue))
      (:`B`
        (set `/Game/Mytaverse/TransformGizmo/BP_TransformGizmo.bEnableLocationSnap` false _returnvalue)
        (set `/Game/Mytaverse/TransformGizmo/BP_TransformGizmo.bEnableRotationSnap` false _returnvalue)
        (set `/Game/Mytaverse/TransformGizmo/BP_TransformGizmo.bEnableScaleSnap` false _returnvalue)))))

(event `self.ReceiveEndPlay`
  (params (EndPlayReason :type "EEndPlayReason Enum" :default "Destroyed"))
  (`KismetSystemLibrary.ExecuteConsoleCommand` "r.AntiAliasingMethod 4" null)
  (`KismetSystemLibrary.ExecuteConsoleCommand` "r.DefaultFeature.AutoExposure 0" null)
  (`KismetSystemLibrary.ExecuteConsoleCommand` "r.MotionBlur.Amount 0" null))

(fn `UserConstructionScript`)