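; Test pawn for the transform gizmo, with an orbit, pan and zoom camera and an on-screen test widget.
; A multi-hit PointerInteraction handles left-click, delaying presses briefly for mobile, and blocks camera input while dragging.
; Hotkeys find BP_TransformGizmo to switch transform mode and toggle align space or snapping.
; BeginPlay turns off anti-aliasing, auto exposure and motion blur via console commands, and EndPlay resets only anti-aliasing.
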(event `self.ReceiveBeginPlay`
  (`parent.ReceiveBeginPlay`)
  (`KismetSystemLibrary.ExecuteConsoleCommand` "r.AntiAliasingMethod 0" null)
  (`KismetSystemLibrary.ExecuteConsoleCommand` "r.DefaultFeature.AutoExposure 0" null)
  (`KismetSystemLibrary.ExecuteConsoleCommand` "r.MotionBlur.Amount 0" null)
  (`/Game/PointerInteraction/BP_PointerInteractionComponent.SetupInteraction` (`self.PointerInteraction`) (make `/Game/PointerInteraction/FPointerInteractionSettings` "NewEnumerator9" 100000.0 true (`|MakeArray` "ObjectTypeQuery2" :!type "EObjectTypeQuery Enum") null) true)
  (bind _returnvalue (`|CreateWidget` "/Game/TransformGizmo/Test/WBP_TransformGizmoTest.WBP_TransformGizmoTest_C"))
  (`UserWidget.AddToViewport` _returnvalue 0))

(event `self.ReceiveTick`
  (params (DeltaSeconds :type "Float (single-precision)"))
  (`parent.ReceiveTick` DeltaSeconds)
  (if (not (`/Game/PointerInteraction/BP_PointerInteractionComponent.bIsDragging` (`self.PointerInteraction`)))
    (`|ExecutionSequence`
      (:`then_0`
        (if (`self.bRightMosuePressed`)
          (`self.AddOrbitInput` (`KismetMathLibrary.MakeVector2D` (`self.GetInputAxisKeyValue`) (`self.GetInputAxisKeyValue`)))
          (elif (`self.bMiddleMousePressed`)
            (`self.AddPanInput` (`KismetMathLibrary.MakeVector2D` (`self.GetInputAxisKeyValue`) (`self.GetInputAxisKeyValue`))))))
      (:`then_1`
        (`self.AddZoomInput` (`self.GetInputAxisKeyValue`))))))

(event `Key|RightMouseButton`
  (params (Key :type "Key Structure"))
  (:`Pressed`
    (set `self.bRightMosuePressed` true))
  (:`Released`
    (set `self.bRightMosuePressed` false)))

(event `Key|MiddleMouseButton`
  (params (Key :type "Key Structure"))
  (:`Pressed`
    (set `self.bMiddleMousePressed` true))
  (:`Released`
    (set `self.bMiddleMousePressed` false)))

(event `self.ReceiveEndPlay`
  (params (EndPlayReason :type "EEndPlayReason Enum" :default "Destroyed"))
  (`KismetSystemLibrary.ExecuteConsoleCommand` "r.AntiAliasingMethod 4" null)
  (`KismetSystemLibrary.ExecuteConsoleCommand` "r.DefaultFeature.AutoExposure 0" null)
  (`KismetSystemLibrary.ExecuteConsoleCommand` "r.MotionBlur.Amount 0" null))

(event `Key|LeftMouseButton`
  (params (Key :type "Key Structure"))
  (bind _pointerinteraction (`self.PointerInteraction`))
  (:`Pressed`
    (`KismetSystemLibrary.Delay` 0.02) ; 方便在移动端也可以使用
    (`/Game/PointerInteraction/BP_PointerInteractionComponent.PressPointer` _pointerinteraction))
  (:`Released`
    (`/Game/PointerInteraction/BP_PointerInteractionComponent.ReleasePointer` _pointerinteraction)))

(event `Key|W`
  (params (Key :type "Key Structure"))
  (:`Pressed`
    (bind _returnvalue (`GameplayStatics.GetActorOfClass` "/Game/TransformGizmo/BP_TransformGizmo.BP_TransformGizmo_C"))
    (`/Game/TransformGizmo/BP_TransformGizmo.SetTransformMode` _returnvalue "NewEnumerator0" false)))

(event `Key|E`
  (params (Key :type "Key Structure"))
  (:`Pressed`
    (bind _returnvalue (`GameplayStatics.GetActorOfClass` "/Game/TransformGizmo/BP_TransformGizmo.BP_TransformGizmo_C"))
    (`/Game/TransformGizmo/BP_TransformGizmo.SetTransformMode` _returnvalue "NewEnumerator1" false)))

(event `Key|R`
  (params (Key :type "Key Structure"))
  (:`Pressed`
    (bind _returnvalue (`GameplayStatics.GetActorOfClass` "/Game/TransformGizmo/BP_TransformGizmo.BP_TransformGizmo_C"))
    (`/Game/TransformGizmo/BP_TransformGizmo.SetTransformMode` _returnvalue "NewEnumerator2" false)))

(event `Key|T`
  (params (Key :type "Key Structure"))
  (:`Pressed`
    (bind _returnvalue (`GameplayStatics.GetActorOfClass` "/Game/TransformGizmo/BP_TransformGizmo.BP_TransformGizmo_C"))
    (`/Game/TransformGizmo/BP_TransformGizmo.SetTransformMode` _returnvalue "NewEnumerator0" true)))

(event `Key|Q`
  (params (Key :type "Key Structure"))
  (:`Pressed`
    (bind _returnvalue (`GameplayStatics.GetActorOfClass` "/Game/TransformGizmo/BP_TransformGizmo.BP_TransformGizmo_C"))
    (`/Engine/EditorBlueprintResources/StandardMacros.FlipFlop`
      (:`A`
        (`/Game/TransformGizmo/BP_TransformGizmo.SetAlignSpace` _returnvalue "NewEnumerator1"))
      (:`B`
        (`/Game/TransformGizmo/BP_TransformGizmo.SetAlignSpace` _returnvalue "NewEnumerator0")))))

(event `Key|S`
  (params (Key :type "Key Structure"))
  (:`Pressed`
    (bind _returnvalue (`GameplayStatics.GetActorOfClass` "/Game/TransformGizmo/BP_TransformGizmo.BP_TransformGizmo_C"))
    (`/Engine/EditorBlueprintResources/StandardMacros.FlipFlop`
      (:`A`
        (set `/Game/TransformGizmo/BP_TransformGizmo.bEnableLocationSnap` true _returnvalue)
        (set `/Game/TransformGizmo/BP_TransformGizmo.bEnableRotationSnap` true _returnvalue)
        (set `/Game/TransformGizmo/BP_TransformGizmo.bEnableScaleSnap` true _returnvalue))
      (:`B`
        (set `/Game/TransformGizmo/BP_TransformGizmo.bEnableLocationSnap` false _returnvalue)
        (set `/Game/TransformGizmo/BP_TransformGizmo.bEnableRotationSnap` false _returnvalue)
        (set `/Game/TransformGizmo/BP_TransformGizmo.bEnableScaleSnap` false _returnvalue)))))

(fn `UserConstructionScript`
  (`parent.UserConstructionScript`))