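; Orbit camera pawn with orbit, pan and zoom (by distance or focal length), limited by yaw, pitch and zoom settings.
; Input events scale deltas by viewport scale; Tick applies them to target values while Orbiting, then interpolates the actor and camera toward those targets.
; StartCameraTransition moves to new settings by timeline blend, fade, teleport or interpolation.
; Optional autofocus line-traces forward to set manual focus distance.
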(event `AddOrbitInput`
  (params (DeltaOrbitInput :type "Vector2D Structure"))
  ;[1 1 1] 输入
  (set `self.DeltaOrbitInput` (* DeltaOrbitInput (/ (`self.CameraOrbitRate`) (`WidgetLayoutLibrary.GetViewportScale`)))))

(event `self.ReceiveBeginPlay`
  (`|ExecutionSequence`
    (:`then_0`
      (set `PlayerController.bShowMouseCursor` true (`GameplayStatics.GetPlayerController` 0)))
    (:`then_1`
      (`self.SetEnableAutoFocus` (`self.bEnableAutoFocus`)))))

(event `AddZoomInput`
  (params (DeltaZoomInput :type "Float (double-precision)"))
  ;[1 1 1] 输入
  (set `self.DeltaZoomInput` (* DeltaZoomInput (`self.GetZoomDistance`) (`self.CameraZoomRate`) (/ -1.0 (`WidgetLayoutLibrary.GetViewportScale`)))))

(event `self.ReceiveTick`
  (params (DeltaSeconds :type "Float (single-precision)"))
  (`|ExecutionSequence`
    (:`then_0`
      (switch `/Game/OrbitCamera/EOrbitCameraState` (`self.OrbitCameraState`)
        (:`NewEnumerator0`
          (`self.HandleOrbitInput`)
          (`self.HandleZoomInput`)
          (`self.HandlePanInput`))))
    (:`then_1`
      (`self.UpdateSmoothMovement` DeltaSeconds))
    (:`then_2`
      (if (`self.bEnableAutoFocus`)
        (`self.UpdateFocusDistance`)))))

(event `AddPanInput`
  (params (DeltaPanInput :type "Vector2D Structure"))
  ;[1 1 1] 输入
  (set `self.DeltaPanInput` (* DeltaPanInput (* (`self.GetZoomDistance`) (`self.CameraPanRate`) (/ -1.0 (`WidgetLayoutLibrary.GetViewportScale`))))))

(event `StartCameraTransition`
  (params (TransitionSettings :type "/Game/OrbitCamera/FOrbitCameraSettings Structure"))
  (bind ((`OrbitLocation_48_BF1412AF49F7725AD2EEBBBF5DC15FD3` _orbitlocation) (`OrbitRotation_16_A6D3FB754BC64E94A4C37EB25A076BCB` _orbitrotation) (`ZoomDistance_7_4B8FF0D84D06DB56580A7CADC89D6A89` _zoomdistance) (`FocalLength_27_A06297E0472BF47126912399589F048A` _focallength) (`HorizontalViewOffset_46_00C32B0C4CA7D53E83A48AA49B3AFD8A` _horizontalviewoffset) (`VerticalViewOffset_47_0A806D5C45F196B6D31DFEAA373C66B9` _verticalviewoffset)) (break `/Game/OrbitCamera/FOrbitCameraSettings` (`self.OrbitCameraSettings`)))
  (bind ((`OrbitLocation_48_BF1412AF49F7725AD2EEBBBF5DC15FD3` _orbitlocation_2) (`OrbitRotation_16_A6D3FB754BC64E94A4C37EB25A076BCB` _orbitrotation_2) (`ZoomDistance_7_4B8FF0D84D06DB56580A7CADC89D6A89` _zoomdistance_2) (`FocalLength_27_A06297E0472BF47126912399589F048A` _focallength_2) (`HorizontalViewOffset_46_00C32B0C4CA7D53E83A48AA49B3AFD8A` _horizontalviewoffset_2) (`VerticalViewOffset_47_0A806D5C45F196B6D31DFEAA373C66B9` _verticalviewoffset_2)) (break `/Game/OrbitCamera/FOrbitCameraSettings` (`self.OrbitCameraSettings`)))
  (bind ((`OrbitLocation_48_BF1412AF49F7725AD2EEBBBF5DC15FD3` _orbitlocation_3) (`OrbitRotation_16_A6D3FB754BC64E94A4C37EB25A076BCB` _orbitrotation_3) (`ZoomDistance_7_4B8FF0D84D06DB56580A7CADC89D6A89` _zoomdistance_3) (`FocalLength_27_A06297E0472BF47126912399589F048A` _focallength_3) (`HorizontalViewOffset_46_00C32B0C4CA7D53E83A48AA49B3AFD8A` _horizontalviewoffset_3) (`VerticalViewOffset_47_0A806D5C45F196B6D31DFEAA373C66B9` _verticalviewoffset_3)) (break `/Game/OrbitCamera/FOrbitCameraSettings` (`self.OrbitCameraSettings`)))
  (bind ((`OrbitLocation_48_BF1412AF49F7725AD2EEBBBF5DC15FD3` _orbitlocation_4) (`OrbitRotation_16_A6D3FB754BC64E94A4C37EB25A076BCB` _orbitrotation_4) (`ZoomDistance_7_4B8FF0D84D06DB56580A7CADC89D6A89` _zoomdistance_4) (`FocalLength_27_A06297E0472BF47126912399589F048A` _focallength_4) (`HorizontalViewOffset_46_00C32B0C4CA7D53E83A48AA49B3AFD8A` _horizontalviewoffset_4) (`VerticalViewOffset_47_0A806D5C45F196B6D31DFEAA373C66B9` _verticalviewoffset_4)) (break `/Game/OrbitCamera/FOrbitCameraSettings` (`self.OrbitCameraSettings`)))
  ;[1 1 1] 相机切换
  (set `self.OrbitCameraSettings` TransitionSettings)
  (set `self.OrbitCameraState` "NewEnumerator1")
  (set `self.TransitionStartLocation` (`self.TargetOrbitLocation`))
  (set `self.TransitionStartRotation` (`self.TargetOrbitRotation`))
  (set `self.TransitionStartFocalLength` (`self.TargetFocalLength`))
  (set `self.TransitionStartZoomDistance` (`self.TargetZoomDistance`))
  (set `self.TransitionStartViewOffset` (`self.TargetViewOffset`))
  (`self.OnTransitionStart`)
  (switch `/Game/OrbitCamera/ETransitionType` (`.TransitionType_24_0A14200340EC8553E82FE3A84AF90F12` (break `/Game/OrbitCamera/FOrbitCameraSettings` (`self.OrbitCameraSettings`)))
    (:`NewEnumerator0`
      (`TimelineComponent.SetPlayRate` (`self.TransitionTimeline`) (`.TimelineRate_40_D4688BC14A2F9C254ED7E8881A1A7F2B` (break `/Game/OrbitCamera/FOrbitCameraSettings` (`self.OrbitCameraSettings`))))
      (bind (_direction _alpha) (`Timeline|TransitionTimeline` :!via `PlayFromStart`)
        (:`Update`
          (set `self.TargetOrbitLocation` (`KismetMathLibrary.VLerp` (`self.TransitionStartLocation`) _orbitlocation_4 _alpha))
          (set `self.TargetOrbitRotation` (`self.LerpRotatorWithoutRoll` (`self.TransitionStartRotation`) _orbitrotation_4 _alpha))
          (set `self.TargetZoomDistance` (`KismetMathLibrary.Lerp` (`self.TransitionStartZoomDistance`) _zoomdistance_4 _alpha))
          (set `self.TargetFocalLength` (`KismetMathLibrary.Lerp` (`self.TransitionStartFocalLength`) _focallength_4 _alpha))
          (set `self.TargetViewOffset` (`KismetMathLibrary.Conv_VectorToVector2D` (`KismetMathLibrary.VLerp` (`KismetMathLibrary.Conv_Vector2DToVector` (`self.TransitionStartViewOffset`)) (`KismetMathLibrary.Conv_Vector2DToVector` (`KismetMathLibrary.MakeVector2D` _horizontalviewoffset_4 _verticalviewoffset_4)) _alpha))))
        (:`Finished`
          (set `self.OrbitCameraState` "NewEnumerator0")
          (`self.OnTransitionFinished`))))
    (:`NewEnumerator1`
      (`|ExecutionSequence`
        (:`then_0`
          (bind _output_get (set `self.TargetOrbitLocation` _orbitlocation_2 :!label _label))
          (set `self.SmoothedOrbitLocation` _output_get)
          (bind _output_get_2 (set `self.TargetOrbitRotation` _orbitrotation_2))
          (set `self.SmoothedOrbitRotation` _output_get_2)
          (bind _output_get_3 (set `self.TargetZoomDistance` _zoomdistance_2))
          (set `self.SmoothedZoomDistance` _output_get_3)
          (bind _output_get_4 (set `self.TargetFocalLength` _focallength_2))
          (set `self.SmoothedFocalLength` _output_get_4)
          (bind _output_get_5 (set `self.TargetViewOffset` (`KismetMathLibrary.MakeVector2D` _horizontalviewoffset_2 _verticalviewoffset_2)))
          (set `self.SmoothedViewOffset` _output_get_5)
          (`PlayerCameraManager.StartCameraFade` :`self` (`GameplayStatics.GetPlayerCameraManager` 0) :`FromAlpha` 1.0 :`Duration` 0.5 :`bHoldWhenFinished` true)
          (set `self.OrbitCameraState` "NewEnumerator0")
          (`self.OnTransitionFinished`))
        (:`then_1`
          (`self.StopTransitionTimeline`))))
    (:`NewEnumerator3`
      (`|ExecutionSequence`
        (:`then_0`
          (`PlayerCameraManager.StartCameraFade` :`self` (`GameplayStatics.GetPlayerCameraManager` 0) :`ToAlpha` 1.0 :`Duration` 0.5 :`bHoldWhenFinished` true)
          (`KismetSystemLibrary.Delay` 0.5)
          (goto _label))
        (:`then_1`
          (`self.StopTransitionTimeline`))))
    (:`NewEnumerator2`
      (`|ExecutionSequence`
        (:`then_0`
          (bind _output_get_6 (set `self.TargetOrbitLocation` _orbitlocation))
          (set `self.SmoothedOrbitLocation` _output_get_6)
          (bind _output_get_7 (set `self.TargetOrbitRotation` _orbitrotation))
          (set `self.SmoothedOrbitRotation` _output_get_7)
          (bind _output_get_8 (set `self.TargetZoomDistance` _zoomdistance))
          (set `self.SmoothedZoomDistance` _output_get_8)
          (bind _output_get_9 (set `self.TargetFocalLength` _focallength))
          (set `self.SmoothedFocalLength` _output_get_9)
          (bind _output_get_10 (set `self.TargetViewOffset` (`KismetMathLibrary.MakeVector2D` _horizontalviewoffset _verticalviewoffset)))
          (set `self.SmoothedViewOffset` _output_get_10)
          (set `self.OrbitCameraState` "NewEnumerator0")
          (`self.OnTransitionFinished`))
        (:`then_1`
          (`self.StopTransitionTimeline`))))
    (:`NewEnumerator5`
      (`|ExecutionSequence`
        (:`then_0`
          (set `self.TargetOrbitLocation` _orbitlocation_3)
          (set `self.TargetOrbitRotation` _orbitrotation_3)
          (set `self.TargetZoomDistance` _zoomdistance_3)
          (set `self.TargetFocalLength` _focallength_3)
          (set `self.TargetViewOffset` (`KismetMathLibrary.MakeVector2D` _horizontalviewoffset_3 _verticalviewoffset_3))
          (set `self.OrbitCameraState` "NewEnumerator0")
          (`self.OnTransitionFinished`))
        (:`then_1`
          (`self.StopTransitionTimeline`))))))

(fn `GetCameraState`
  (returns (ReturnValue :type "/Game/OrbitCamera/EOrbitCameraState Enum"))
  (return (`self.OrbitCameraState`)))

(fn `GetFocalLength`
  (returns (ReturnValue :type "Float (double-precision)"))
  (return (`CineCameraComponent.CurrentFocalLength` (`self.OrbitCamera`))))

(fn `GetZoomDistance`
  (returns (ReturnValue :type "Float (double-precision)"))
  (return (`KismetMathLibrary.VSize` (`SceneComponent.RelativeLocation` (`self.OrbitCamera`)))))

(fn `HandleOrbitInput`
  (bind ((`MinPitchOffset_11_D0442B41432140C6800E259F95B0B024` _minpitchoffset) (`MaxPitchOffset_9_73C35D5042549E9F5BBFA6AB8DF0136F` _maxpitchoffset)) (break `/Game/OrbitCamera/FOrbitCameraSettings` (`self.OrbitCameraSettings`)))
  (bind (_x _y) (`KismetMathLibrary.BreakVector2D` (`self.DeltaOrbitInput`)))
  (set `self.TargetOrbitRotation` (`KismetMathLibrary.MakeRotator` 0.0 (`KismetMathLibrary.ClampAngle` (`KismetMathLibrary.ClampAngle` (+ (.pitch (`self.TargetOrbitRotation`)) (`KismetMathLibrary.SelectFloat` _y 0.0 (`self.IsPendingPitchInRange` _y))) _minpitchoffset _maxpitchoffset) -89.9 89.9) (+ (.yaw (`self.TargetOrbitRotation`)) (`KismetMathLibrary.SelectFloat` _x 0.0 (`self.IsPendingYawInRange` _x)))))
  (set `self.DeltaOrbitInput` (0.0 0.0)) ; 需要归零
)

(fn `HandlePanInput`
  (bind (_deltapaninput_x _deltapaninput_y) (`KismetMathLibrary.BreakVector2D` (`self.DeltaPanInput`)))
  (set `self.TargetOrbitLocation` (+ (`self.TargetOrbitLocation`) (+ (* (`KismetMathLibrary.SelectVector` (`KismetMathLibrary.GetForwardVector` (`KismetMathLibrary.MakeRotFromYZ` (`self.GetActorRightVector`) (`KismetMathLibrary.Vector_Up`))) (`self.GetActorUpVector`) (`self.bPanHorizontally`)) _deltapaninput_y) (* (`self.GetActorRightVector`) _deltapaninput_x))))
  (set `self.DeltaPanInput` (0.0 0.0)))

(fn `HandleZoomInput`
  (bind _deltazoominput (`self.DeltaZoomInput`))
  (bind ((`MinZoomDistance_19_A3E0168948445E0A3FE20DB3DA3F2692` _minzoomdistance) (`MaxZoomDistance_21_52D528BC4D33907BF4EE8D857F2749BC` _maxzoomdistance)) (break `/Game/OrbitCamera/FOrbitCameraSettings` (`self.OrbitCameraSettings`)))
  (bind ((`MinFocalLength_33_7172CF0C413F2636C0DA98884F0D149D` _minfocallength) (`MaxFocalLength_35_924D1DF54DF72E6CC4E340B4BD34427D` _maxfocallength) (`bUseFocalZoom_37_AB297E494D5FC0596FB5B4BC1B5A0026` _busefocalzoom)) (break `/Game/OrbitCamera/FOrbitCameraSettings` (`self.OrbitCameraSettings`)))
  (if _busefocalzoom
    (set `self.TargetFocalLength` (`KismetMathLibrary.FClamp` (+ (`self.TargetFocalLength`) (* _deltazoominput -1.0)) _minfocallength _maxfocallength))
    (else
      (set `self.TargetZoomDistance` (`KismetMathLibrary.FClamp` (+ (`self.TargetZoomDistance`) _deltazoominput) _minzoomdistance _maxzoomdistance))))
  (set `self.DeltaZoomInput` 0.0))

(fn `IsPendingPitchInRange`
  (params (DeltaPitch :type "Float (double-precision)"))
  (returns (ReturnValue :type Boolean))
  (bind ((`ConstraintBaseAxis_30_0813F23F42FBE5DC2ECB2BBAD3C85AD1` _constraintbaseaxis) (`MinPitchOffset_11_D0442B41432140C6800E259F95B0B024` _minpitchoffset) (`MaxPitchOffset_9_73C35D5042549E9F5BBFA6AB8DF0136F` _maxpitchoffset)) (break `/Game/OrbitCamera/FOrbitCameraSettings` (`self.OrbitCameraSettings`)))
  (bind (_returnvalue_roll _returnvalue_pitch) (`KismetMathLibrary.BreakRotator` (`KismetMathLibrary.Conv_VectorToRotator` _constraintbaseaxis)))
  (bind (_returnvalue_x _returnvalue_y _returnvalue_z) (`KismetMathLibrary.BreakVector` (`KismetMathLibrary.GetForwardVector` (`KismetMathLibrary.MakeRotator` 0.0 _returnvalue_pitch))))
  (bind (_returnvalue_x_2 _returnvalue_y_2 _returnvalue_z_2) (`KismetMathLibrary.BreakVector` (`KismetMathLibrary.GetForwardVector` (`KismetMathLibrary.ComposeRotators` (`KismetMathLibrary.MakeRotator` 0.0 (.pitch (`self.TargetOrbitRotation`))) (`KismetMathLibrary.MakeRotator` 0.0 DeltaPitch)))))
  (bind _returnvalue (`KismetMathLibrary.MakeVector2D` _returnvalue_x_2 _returnvalue_z_2))
  (bind _returnvalue_2 (`KismetMathLibrary.MakeVector2D` _returnvalue_x _returnvalue_z))
  (return (`KismetMathLibrary.InRange_FloatFloat` (* (`KismetMathLibrary.DegAcos` (`KismetMathLibrary.DotProduct2D` _returnvalue_2 _returnvalue)) (`KismetMathLibrary.SignOfFloat` (`KismetMathLibrary.CrossProduct2D` _returnvalue_2 _returnvalue))) _minpitchoffset _maxpitchoffset)))

(fn `IsPendingYawInRange`
  (params (DeltaYaw :type "Float (double-precision)"))
  (returns (ReturnValue :type Boolean))
  (bind ((`ConstraintBaseAxis_30_0813F23F42FBE5DC2ECB2BBAD3C85AD1` _constraintbaseaxis) (`MinYawOffset_15_7843FB164D843CCDEF238686AD339BBA` _minyawoffset) (`MaxYawOffset_13_A6EDD8D345C4E2DD8A999DACA0CDAE2D` _maxyawoffset)) (break `/Game/OrbitCamera/FOrbitCameraSettings` (`self.OrbitCameraSettings`)))
  (bind _returnvalue (`KismetMathLibrary.Normal2D` (`KismetMathLibrary.Conv_VectorToVector2D` _constraintbaseaxis)))
  (bind _returnvalue_2 (`KismetMathLibrary.Normal2D` (`KismetMathLibrary.Conv_VectorToVector2D` (`KismetMathLibrary.GetForwardVector` (`KismetMathLibrary.ComposeRotators` (`self.TargetOrbitRotation`) (`KismetMathLibrary.MakeRotator` 0.0 0.0 DeltaYaw))))))
  (return (`KismetMathLibrary.InRange_FloatFloat` (* (`KismetMathLibrary.DegAcos` (`KismetMathLibrary.DotProduct2D` _returnvalue _returnvalue_2)) (`KismetMathLibrary.SignOfFloat` (`KismetMathLibrary.CrossProduct2D` _returnvalue _returnvalue_2))) _minyawoffset _maxyawoffset)))

(fn `LerpRotatorWithoutRoll`
  (params (A :type "Rotator Structure") (B :type "Rotator Structure") (Alpha :type "Float (double-precision)"))
  (returns (ReturnValue :type "Rotator Structure"))
  (bind (_returnvalue_roll _returnvalue_pitch _returnvalue_yaw) (`KismetMathLibrary.BreakRotator` (`KismetMathLibrary.RLerp` (`KismetMathLibrary.MakeRotator` 0.0 A_Pitch A_Yaw) (`KismetMathLibrary.MakeRotator` 0.0 B_Pitch B_Yaw) Alpha true)))
  (return (`KismetMathLibrary.MakeRotator` 0.0 _returnvalue_pitch _returnvalue_yaw)))

(fn `SetEnableAutoFocus`
  (params (bEnabled :type Boolean))
  (bind _output_get (set `self.bEnableAutoFocus` bEnabled))
  (setmembers `CameraFocusSettings` :`StructRef` (`CineCameraComponent.FocusSettings` (`self.OrbitCamera`)) :`FocusMethod` (select `bool` _output_get :`false` "Disable" :`true` "Manual" :!type "ECameraFocusMethod Enum") :`bSmoothFocusChanges` true))

(fn `SetFocalLength`
  (params (InFocalLength :type "Float (double-precision)"))
  (set `CineCameraComponent.CurrentFocalLength` InFocalLength (`self.OrbitCamera`)))

(fn `SetZoomDistance`
  (params (InZoomDistance :type "Float (double-precision)"))
  (bind (_smoothedviewoffset_x _smoothedviewoffset_y) (`KismetMathLibrary.BreakVector2D` (`self.SmoothedViewOffset`)))
  (`SceneComponent.K2_SetRelativeLocation` (`self.OrbitCamera`) (`KismetMathLibrary.NegateVector` (`KismetMathLibrary.CreateVectorFromYawPitch` _smoothedviewoffset_x _smoothedviewoffset_y InZoomDistance)) false false))

(fn `StopTransitionTimeline`
  (bind _transitiontimeline (`self.TransitionTimeline`))
  (if (`TimelineComponent.IsPlaying` _transitiontimeline)
    (`TimelineComponent.Stop` _transitiontimeline)))

(fn `UpdateFocusDistance`
  (bind _orbitcamera (`self.OrbitCamera`))
  (bind _returnvalue (`SceneComponent.K2_GetComponentLocation` _orbitcamera))
  (bind (_outhit _returnvalue_2) (`KismetSystemLibrary.LineTraceSingle` _returnvalue (+ _returnvalue (* (`SceneComponent.GetForwardVector` _orbitcamera) 2000.0)) "TraceTypeQuery1" true))
  (if _returnvalue_2
    (setmembers `CameraFocusSettings` :`StructRef` (`CineCameraComponent.FocusSettings` (`self.OrbitCamera`)) :`ManualFocusDistance` (`.Distance` (`GameplayStatics.BreakHitResult` _outhit)))))

(fn `UpdateSmoothMovement`
  (params (DeltaTime :type "Float (double-precision)"))
  (set `self.SmoothedOrbitLocation` (`KismetMathLibrary.VInterpTo` (`self.SmoothedOrbitLocation`) (`self.TargetOrbitLocation`) DeltaTime (`self.SmoothInterpSpeed`)))
  (set `self.SmoothedOrbitRotation` (`KismetMathLibrary.RInterpTo` (`self.SmoothedOrbitRotation`) (`self.TargetOrbitRotation`) DeltaTime (`self.SmoothInterpSpeed`)))
  (`self.K2_SetActorLocationAndRotation` (`self.SmoothedOrbitLocation`) (`self.SmoothedOrbitRotation`))
  (bind _output_get (set `self.SmoothedFocalLength` (`KismetMathLibrary.FInterpTo` (`self.SmoothedFocalLength`) (`self.TargetFocalLength`) DeltaTime (`self.SmoothInterpSpeed`))))
  (`self.SetFocalLength` _output_get)
  (set `self.SmoothedViewOffset` (`KismetMathLibrary.Vector2DInterpTo` (`self.SmoothedViewOffset`) (`self.TargetViewOffset`) DeltaTime (`self.SmoothInterpSpeed`)))
  (bind _output_get_2 (set `self.SmoothedZoomDistance` (`KismetMathLibrary.FInterpTo` (`self.SmoothedZoomDistance`) (`self.TargetZoomDistance`) DeltaTime (`self.SmoothInterpSpeed`))))
  (`self.SetZoomDistance` _output_get_2))

(fn `UserConstructionScript`
  (bind _returnvalue (`self.K2_GetActorRotation`))
  (bind (_returnvalue_roll _returnvalue_pitch _returnvalue_yaw) (`KismetMathLibrary.BreakRotator` (`self.K2_GetActorRotation`)))
  (bind ((`ZoomDistance_7_4B8FF0D84D06DB56580A7CADC89D6A89` _zoomdistance) (`FocalLength_27_A06297E0472BF47126912399589F048A` _focallength)) (break `/Game/OrbitCamera/FOrbitCameraSettings` (`self.OrbitCameraSettings`)))
  (`parent.UserConstructionScript`)
  (`|ExecutionSequence`
    (:`then_0`
      (`self.SetZoomDistance` _zoomdistance)
      (set `self.TargetZoomDistance` _zoomdistance)
      (`self.SetFocalLength` _focallength)
      (set `self.TargetFocalLength` _focallength)
      (`self.K2_SetActorRotation` (`KismetMathLibrary.MakeRotator` 0.0 _returnvalue_pitch _returnvalue_yaw)))
    (:`then_1`
      (setmembers `/Game/OrbitCamera/FOrbitCameraSettings` :`StructRef` (`self.OrbitCameraSettings`) :`OrbitLocation` (`self.K2_GetActorLocation`) :`OrbitRotation` _returnvalue :`ConstraintBaseAxis` (`KismetMathLibrary.Conv_RotatorToVector` (`KismetMathLibrary.MakeRotator` 0.0 0.0 (.yaw _returnvalue))))
      (set `self.TargetOrbitRotation` (`self.K2_GetActorRotation`))
      (set `self.TargetOrbitLocation` (`self.K2_GetActorLocation`)))))